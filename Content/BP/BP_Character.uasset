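; BP_Character is a player character Blueprint that provides basic movement, camera look and jumping from input.
; Forward and right axis inputs add movement relative to control rotation: forward uses only yaw, while right uses yaw and roll.
; Mouse axes drive controller pitch and yaw, and the Jump action starts and stops jumping on press and release.
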(event Input|ActionEvents|InputActionJump
  (params (Key :type Key%20Structure :default "None"))
  ;[1 1 1] Salto
  (:Pressed
    (Character|Jump))
  (:Released
    (Character|StopJumping)))

(event Input|AxisEvents|InputAxisMoveForward
  (params (AxisValue :type Float%20%28single-precision%29))
  ;[1 1 1] mover adelante y atras
  (Pawn|Input|AddMovementInput (Math|Vector|GetForwardVector (Math|Rotator|MakeRotator 0.0 0.0 (.yaw (Pawn|GetControlRotation :!class /Script/Engine.Pawn)))) AxisValue false))

(event Input|AxisEvents|InputAxisMoveRight
  (params (AxisValue :type Float%20%28single-precision%29))
  (bind _returnvalue (Pawn|GetControlRotation :!class /Script/Engine.Pawn))
  ;[1 1 1] mover derecha e izquierda
  (Pawn|Input|AddMovementInput (Math|Vector|GetRightVector (Math|Rotator|MakeRotator (.roll _returnvalue) 0.0 (.yaw _returnvalue))) AxisValue false))

(event Input|AxisEvents|InputAxisMouseUpDown
  (params (AxisValue :type Float%20%28single-precision%29))
  ;[1 1 1] arriba y abajo de la camara
  (Pawn|Input|AddControllerPitchInput AxisValue))

(event Input|AxisEvents|InputAxisMouseRightLeft
  (params (AxisValue :type Float%20%28single-precision%29))
  ;[1 1 1] izq y der camara
  (Pawn|Input|AddControllerYawInput AxisValue))

(fn ConstructionScript)